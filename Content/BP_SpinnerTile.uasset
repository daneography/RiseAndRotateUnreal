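; BP_SpinnerTile is a tile actor that lifts, turns and lowers on numpad input, which it enables on BeginPlay.
; NumPad 4 and 6 each chain Rise, RotateLeft or RotateRight, and Fall, spaced by one-second delays.
; Rise and Fall offset the Spinner component vertically, while rotation yaws the whole actor in 45-degree steps, all as instant jumps.
; An unconnected loop repeating the right-turn sequence never runs.
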(event `self.ReceiveBeginPlay`
  (`self.EnableInput` (`GameplayStatics.GetPlayerController` 0)))

(event `self.ReceiveTick`
  (params (DeltaSeconds :type "Float (single-precision)")))

(event `Rise`
  (`SceneComponent.K2_AddRelativeLocation` (`self.Spinner`) (`KismetMathLibrary.MakeVector` 0.0 0.0 100.0) false false))

(event `RotateLeft`
  (`self.K2_AddActorLocalRotation` (`KismetMathLibrary.MakeRotator` 0.0 0.0 45.0)))

(event `RotateRight`
  (`self.K2_AddActorLocalRotation` (`KismetMathLibrary.MakeRotator` 0.0 0.0 -45.0)))

(event `Fall`
  (`SceneComponent.K2_AddRelativeLocation` (`self.Spinner`) (`KismetMathLibrary.MakeVector` 0.0 0.0 -100.0) false false))

(event `Key|NumPadFour`
  (params (Key :type "Key Structure"))
  (:`Pressed`
    (`self.Rise`)
    (`KismetSystemLibrary.Delay` 1.0)
    (`self.RotateLeft`)
    (`KismetSystemLibrary.Delay` 1.0)
    (`self.Fall`)
    (`KismetSystemLibrary.Delay` 1.0)))

(event `Key|NumPadSix`
  (params (Key :type "Key Structure"))
  (:`Pressed`
    (`self.Rise`)
    (`KismetSystemLibrary.Delay` 1.0)
    (`self.RotateRight`)
    (`KismetSystemLibrary.Delay` 1.0)
    (`self.Fall`)
    (`KismetSystemLibrary.Delay` 1.0)))

(fn `UserConstructionScript`)